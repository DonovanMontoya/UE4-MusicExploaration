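; Sound emission cube that plays a looping-style jazz track with spatial attenuation when hit.
; The first hit spawns the sound at the hit location; later hits toggle pause and resume through the IsPaused flag.
; A fixed delay clears SoundOn regardless of pauses, so the next hit spawns a fresh sound.
; Unwired leftover variants hold a stop-toggle block and a one-shot impact sound.
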(event Collision|EventActorBeginOverlap
  (params (OtherActor :type Actor%20Object%20Reference)))

(event Collision|EventHit
  (params (MyComp :type Primitive%20Component%20Object%20Reference) (Other :type Actor%20Object%20Reference) (OtherComp :type Primitive%20Component%20Object%20Reference) (bSelfMoved :type Boolean) (HitLocation :type Vector :default "0, 0, 0") (HitNormal :type Vector :default "0, 0, 0") (NormalImpulse :type Vector :default "0, 0, 0") (Hit :type Hit%20Result%20Structure%20%28by%20ref%29))
  ;[1 1 1] Pausable  -- Works best with loopable audio, as not accounting for audio length
  (if (Variables|Default|GetsoundOn)
    (if (Variables|Default|GetisPaused)
      (Class|AudioComponent|SetPaused (stale _returnvalue) false)
      (Variables|Default|SetisPaused false)
      (else
        (Class|AudioComponent|SetPaused (stale _returnvalue) true)
        (Variables|Default|SetisPaused true)))
    (else
      (Variables|Default|SetsoundOn true)
      (bind _returnvalue (Audio|SpawnSoundatLocation "/Game/Blueprints/SoundObjects/Jazz_tune_A_b.Jazz_tune_A_b" HitLocation "0, 0, 0" 1.0 1.0 0.0 "/Game/Blueprints/SoundObjects/FirstPersonSoundAttenuation.FirstPersonSoundAttenuation" 0))
      (Utilities|FlowControl|Delay 69.0)
      (Variables|Default|SetsoundOn false))))

(fn ConstructionScript)